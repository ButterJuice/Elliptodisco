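; Game mode for an endless runner that manages screen widgets and the chain of spawned floor tiles.
; Screens are looked up by camera-state key in a widget database, created once, cached in a map, and shown after removing the others.
; Each switch sets the pawn's camera state and fires a screen-changed event, which toggles input and gameplay messages and starts tile spawning.
; Tiles chain from attach points; extending adds one and expires the oldest.
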(event Custom|OnWidgetScreenChanged_Event
  (bind _returnvalue (Game|Player|GetPlayerPawn 0))
  (bind _returnvalue_2 (Game|Player|GetPlayerPawn 0))
  (bind _playercontroller (Variables|Default|GetPlayerController))
  ;[0.15 0.15 0.15 0.5] Called everytime a new widget screen is added to viewport, can be extended to execute specific tasks on any screen.
  (if (Utilities|Enum|Equal(Enum) (CallFunction|GetCameraState (Game|Player|GetPlayerPawn 0)) "NewEnumerator15")
    (Input|EnableInput _returnvalue_2 _playercontroller)
    (CallFunction|StartSpawningTiles)
    (Class|BPIPlayerInterface|StartPlayingGame(Message) _returnvalue)
    (else
      (Input|DisableInput _returnvalue_2 _playercontroller)
      (Class|BPIPlayerInterface|StopGameplay(Message) _returnvalue))))

(event Custom|RemoveOnScreenWidgets
  ;[0.15 0.15 0.15 0.5] Avoid Overlapping Widgets
  (bind _valuepin (Utilities|Map|ForEachLoop(Map) (Variables|Default|GetCachedData))
    (:then
      (Utilities|IsValid (.widgetelement _valuepin)
        (:Is%20Valid
          (Widget|RemovefromParent (.widgetelement _valuepin)))))))

(event Custom|StartSpawningTiles
  ;[0.15 0.15 0.15 0.5] Start adding floor tiles as the game begins
  (for _index (range 0 (+ (Variables|Default|GetNumberOfTiles) 4))
    (CallFunction|AddFloor)))

(event EventAddWidgettoScreen
  (params (Screen :type E_WidgetScreen%20Enum :default "NewEnumerator3"))
  ;[0.15 0.15 0.15 0.5] WidgetsManager
  (CallFunction|RemoveonScreenWidgets)
  (CallFunction|CreateWidget Screen))

(event EventBeginPlay
  ;[0.15 0.15 0.15 0.5] Cache for future reference
  (Utilities|FlowControl|Sequence
    (:then_0
      (EventDispatchers|BindEventtoOnWidgetScreenChanged (EventDispatchers|CreateEvent :!event Custom|OnWidgetScreenChanged_Event))
      ;;[0.15 0.15 0.15 0.5] Cache player controller for future reference
      (Variables|Default|SetPlayerController (Game|GetPlayerController 0)))
    (:then_1
      (Variables|Default|SetWidgetsData (Variables|/Game/Runner_Game/WMS/DataAsset/PDA_WidgetData.PDA_WidgetData_C|GetWidgetsData (Variables|Default|GetWidgetDataBase)))
      ;;[0.15 0.15 0.15 0.5] Create Main Menu on BeginPlay
      (CallFunction|CreateWidget "NewEnumerator3"))))

(fn ConstructionScript)

(fn AddFloor
  (bind _returnvalue (Game|SpawnActorfromClass "/Game/Runner_Game/Obstacles/BP_Floor.BP_Floor_C" (Variables|Default|GetFloorAttachPoint) "Undefined" "MultiplyWithRoot" 0 0))
  (Variables|Default|SetFloorAttachPoint (Default|GetAttachPoint _returnvalue))
  (Utilities|Array|Add (Variables|Default|GetFloorTile) _returnvalue))

(fn ExtendFloor
  (CallFunction|AddFloor) ; Add new floor
  (CallFunction|DeleteFloor) ; Delete the last floor
)

(fn DeleteFloor
  (bind _floortile (Variables|Default|GetFloorTile))
  (bind _output (Utilities|Array|Get(acopy) _floortile))
  ;[0.15 0.15 0.15 0.5] Delete the last floor in (lifespan) seconds.
  (Actor|SetLifeSpan _output 3.0)
  (Utilities|Array|RemoveItem _floortile _output))

(fn CreateWidget
  (params (Key :type E_WidgetScreen%20Enum :default "NewEnumerator3"))
  (bind _cacheddata (Variables|Default|GetCachedData))
  (bind (_value _returnvalue) (Utilities|Map|Find _cacheddata Key))
  (if _returnvalue
    (LocalVariables|SetCurrentScreen (.index _value))
    (UserInterface|Viewport|AddtoViewport (.widgetelement _value) 0)
    (CallFunction|ChangeCameraState Key (Game|Player|GetPlayerPawn 0))
    (Default|CallOnWidgetScreenChanged)
    (return)
    (else
      (bind (_array_element _array_index) (Utilities|Array|ForEachLoopwithBreak (Variables|Default|GetWidgetsData) :!label _label)
        (:LoopBody
          (if (Utilities|Enum|Equal(Enum) Key (.CameraState (Utilities|Struct|BreakS_WidgetData _array_element)))
            (LocalVariables|SetCurrentScreen _array_index)
            (goto _label Break)))
        (:Completed
          (if (!= (LocalVariables|GetCurrentScreen) -1)
            (bind _returnvalue_2 (UserInterface|CreateWidget (.widgetelement (Utilities|Array|Get(acopy) (Variables|Default|GetWidgetsData) (LocalVariables|GetCurrentScreen)))))
            (Utilities|Map|Add (Variables|Default|GetCachedData) Key (Utilities|Struct|MakeS_CacheData (LocalVariables|GetCurrentScreen) _returnvalue_2))
            (UserInterface|Viewport|AddtoViewport _returnvalue_2 0)
            (CallFunction|ChangeCameraState Key (Game|Player|GetPlayerPawn 0))
            (Default|CallOnWidgetScreenChanged)
            (return)
            (else
              (Development|PrintString "Requested Widget Screen Not found in database" true true "(R=1.000000,G=0.016108,B=0.000000,A=1.000000)")
              (return))))))))

(fn GetCharacterSelectionWidget
  (bind _cacheddata (Variables|Default|GetCachedData))
  (bind (_value _returnvalue) (Utilities|Map|Find _cacheddata "NewEnumerator20"))
  (if _returnvalue
    (bind _asw_char_select_screen (Utilities|Casting|CastToW_CharSelectScreen (.widgetelement _value))
      (:then
        (return _asw_char_select_screen true))
      (:CastFailed
        (return 0 false)))
    (else
      (return 0 true))))