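; Player controller for the runner game that drives character selection, using a level CameraActor as the view.
; Next and previous events step through a character data list, spawning the chosen pawn at the current one's transform, possessing it and preserving control rotation.
; Range checks set end-of-list flags that block further stepping and are sent to the selection widget obtained from the game mode, after which the player pawn emotes.
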(event EventBeginPlay
  (bind _outactors (Actor|GetAllActorsOfClass "/Script/Engine.CameraActor"))
  (Game|Player|SetViewTargetwithBlend (Utilities|Array|Get(acopy) _outactors) 0.0 "VTBlend_Linear" 0.0 false))

(event EventGetPreviousCharacter
  (params (Idx :type Integer))
  ;[0.15 0.15 0.15 0.5] Character fetch logic in backward direction
  (bind _disableprevbutton (Variables|WMS|GetDisablePrevButton) ; Get if previous button was disabled or not
    (:then
      (Development|PrintString "PrevDisable") ; For Debugging Only - When the button is disabled.
    )
    (:else
      (WMS|GetCharacter Idx)))
  (bind (_widget _valid_) (Class|BPIGameModeInterface|GetCharacterSelectionWidget(Message) (Game|GetGameMode)))
  (if _valid_
    (Class|BPICharSelectInterface|IsPreviousButtonDisabled(Message) _widget _disableprevbutton) ; Manage if or not the button should be disabled
    ;[0.15 0.15 0.15 0.5] Emote here so that any new pawn can emote
    (Default|EmoteNow (Actor|GetComponentbyClass (Game|Player|GetPlayerPawn 0) "/Game/Runner_Game/CCS/Attributes/BPC_PlayerAttributes.BPC_PlayerAttributes_C"))))

(event EventGetNextCharacter
  (params (Idx :type Integer))
  ;[0.15 0.15 0.15 0.5] Character fetch logic in forward direction
  (bind _disablenextbutton (Variables|WMS|GetDisableNextButton)
    (:then
      (Development|PrintString "NextDisable"))
    (:else
      (WMS|GetCharacter Idx)))
  (bind (_widget _valid_) (Class|BPIGameModeInterface|GetCharacterSelectionWidget(Message) (Game|GetGameMode)))
  (if _valid_
    (Class|BPICharSelectInterface|IsNextButtonDisabled(Message) _widget _disablenextbutton)
    ;[0.15 0.15 0.15 0.5] Emote here so that any new pawn can emote
    (Default|EmoteNow (Actor|GetComponentbyClass (Game|Player|GetPlayerPawn 0) "/Game/Runner_Game/CCS/Attributes/BPC_PlayerAttributes.BPC_PlayerAttributes_C"))))

(fn ConstructionScript)

(fn GetCharacter
  (params (Index :type Integer))
  (bind _returnvalue (Pawn|GetControlledPawn))
  (Variables|WMS|SetCurrent%20Character%20Index (Math|Integer|%(Integer) (+ (Variables|WMS|GetCurrent%20Character%20Index) Index) (Utilities|Array|Length (Variables|/Game/Runner_Game/CSS/PDA/PDA_CharacterSelectionData.PDA_CharacterSelectionData_C|GetCharacterData (Variables|WMS|GetCharacter%20Data)))))
  (Utilities|CheckRange)
  (Variables|WMS|SetCachedControlRotation (Pawn|GetControlRotation :!class /Script/Engine.Controller))
  (Variables|IMPORTANT|SetCurrentCharacterData (Utilities|Array|Get(acopy) (Variables|/Game/Runner_Game/CSS/PDA/PDA_CharacterSelectionData.PDA_CharacterSelectionData_C|GetCharacterData (Variables|WMS|GetCharacter%20Data)) (Variables|WMS|GetCurrent%20Character%20Index)))
  (bind _returnvalue_2 (Game|SpawnActorfromClass (Variables|/Game/Runner_Game/CSS/PDA/PDA_CharacterData.PDA_CharacterData_C|GetClass (Utilities|Array|Get(acopy) (Variables|/Game/Runner_Game/CSS/PDA/PDA_CharacterSelectionData.PDA_CharacterSelectionData_C|GetCharacterData (Variables|WMS|GetCharacter%20Data)) (Variables|WMS|GetCurrent%20Character%20Index))) (Transformation|GetActorTransform _returnvalue) "AlwaysSpawn" "MultiplyWithRoot" 0 0))
  (Actor|DestroyActor _returnvalue)
  (Pawn|Possess _returnvalue_2)
  (Pawn|SetControlRotation (Variables|WMS|GetCachedControlRotation)))

(fn GetCharacterData
  (return (Variables|IMPORTANT|GetCurrentCharacterData)))