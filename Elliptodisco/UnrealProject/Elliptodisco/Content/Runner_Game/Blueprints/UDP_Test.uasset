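; Test Blueprint in Runner_Game that receives UDP packets and prints their decoded contents to screen for debugging.
; The first byte is a flag selecting the decoder: 4 reads two button states and a magnet state, 2 reads a speed value.
; Speed is assembled from four little-endian bytes and scaled from microseconds to seconds, though the lowest byte is multiplied by zero and drops out.
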(event OnReceivedBytes(UDP)
  (params (Bytes :type Array%20of%20Bytes) (IPAddress :type String) (Port :type Integer%20%28by%20ref%29))
  (bind _output (Utilities|Array|Get(acopy) Bytes))
  (Development|PrintString (Utilities|String|Append "Flag is : " (Utilities|String|ToString(Byte) (Utilities|Array|Get(acopy) Bytes))))
  ;[0.15 0.15 0.15 0.5] Change comportement according to the flag
  (if (== _output 4)
    (bind (_buttonone _buttontwo _magnetstate) (CallFunction|ReadButtonStates Bytes))
    (Development|PrintString (Utilities|String|Append (Utilities|String|Append (Utilities|String|ToString(Byte) _buttonone) (Utilities|String|ToString(Byte) _buttontwo) (Utilities|String|ToString(Byte) _magnetstate)) ", From IP: " IPAddress))
    (elif (== _output 2)
      (bind _speedfloat (CallFunction|ReadSpeedValue Bytes))
      (Development|PrintString (Utilities|String|Append "Speed : " (Utilities|String|ToString(Float) _speedfloat))))))

(event EventBeginPlay
  (Development|PrintString "Instantiated"))

(event Collision|EventActorBeginOverlap
  (params (OtherActor :type Actor%20Object%20Reference)))

(event EventTick
  (params (DeltaSeconds :type Float%20%28single-precision%29)))

(fn ConstructionScript)

(fn ReadButtonStates
  (params (Buttons :type Array%20of%20Bytes))
  (return (Utilities|Array|Get(acopy) Buttons 1) (Utilities|Array|Get(acopy) Buttons 2) (Utilities|Array|Get(acopy) Buttons 3)))

(fn ReadSpeedValue
  (params (SpeedBytes :type Array%20of%20Bytes))
  (return (/ (+ (* (Math|Conversions|ToFloat(Byte) (Utilities|Array|Get(acopy) SpeedBytes 1)) 0.0) (* (Math|Conversions|ToFloat(Byte) (Utilities|Array|Get(acopy) SpeedBytes 2)) 256.0) (* (Math|Conversions|ToFloat(Byte) (Utilities|Array|Get(acopy) SpeedBytes 3)) 65536.0) (* (Math|Conversions|ToFloat(Byte) (Utilities|Array|Get(acopy) SpeedBytes 4)) 16777216.0)) 1e+06)))