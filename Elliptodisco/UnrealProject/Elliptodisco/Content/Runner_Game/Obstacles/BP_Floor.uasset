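; BP_Floor is a floor tile for an endless runner that places a random obstacle set piece on itself.
; Construction creates one arrow spawn point per LanePosition entry, shuffles them, and attaches one of seven child-actor set pieces at the first, converted to relative space.
; When the Detector is overlapped, it tells BP_RunnerGM to extend the floor and raises the player's walk speed by 10%, clamped to a range.
; GetAttachPoint exposes the AttachPoint world transform.
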(event OnComponentBeginOverlap(Detector)
  (params (OverlappedComponent :type Primitive%20Component%20Object%20Reference) (OtherActor :type Actor%20Object%20Reference) (OtherComp :type Primitive%20Component%20Object%20Reference) (OtherBodyIndex :type Integer) (bFromSweep :type Boolean) (SweepResult :type Hit%20Result%20Structure%20%28by%20ref%29))
  ;[0.15 0.15 0.15 0.5] Detects and validates the player
  (bind _asbp_runner_gm (Utilities|Casting|CastToBP_RunnerGM (Game|GetGameMode)))
  ;[0.15 0.15 0.15 0.5] Function in gamemode that extends the floor ahead of the player
  (Default|ExtendFloor _asbp_runner_gm)
  ;[1 1 1] Change Speed
  (bind _asbp_runner_char_base (Utilities|Casting|CastToBP_RunnerCharBase (Game|GetPlayerCharacter 0)))
  (Variables|/Script/Engine.CharacterMovementComponent|SetMaxWalkSpeed (Variables|/Script/Engine.Character|GetCharacterMovement _asbp_runner_char_base) (Math|Float|Clamp(Float) (* (Variables|/Script/Engine.CharacterMovementComponent|GetMaxWalkSpeed (Variables|/Script/Engine.Character|GetCharacterMovement _asbp_runner_char_base)) 1.1) 8e+02 2e+03)))

(fn ConstructionScript
  (CallFunction|SetSpawnPoints)
  (CallFunction|SpawnObstacles))

(fn GetAttachPoint
  (return (Transformation|GetWorldTransform (Variables|Default|GetAttachPoint))))

(fn SetSpawnPoints
  (for _array_element (Variables|Default|GetLanePosition)
    ;[1 1 1] This loop generates the number of spawn points on the floor. Changing the value last index does the work. Here the function currently spawns a set piece instead of individual obstacles. So, only one spawn point is needed.
    (for _index (range 0 0)
      (bind _returnvalue (AddComponent|AddArrowComponent false (Math|Transform|MakeTransform (Math|Vector|MakeVector 0.0 _array_element 0.0))))
      (Utilities|Array|Add (Variables|Default|GetSpawnPoints) (Transformation|GetWorldTransform _returnvalue)))))

(fn SpawnObstacles
  ;[0.15 0.15 0.15 0.5] Adds randomness in spawning obstacles
  (bind _output_get (LocalVariables|SetRandom%20Spawn%20Points (Variables|Default|GetSpawnPoints)))
  (Utilities|Array|Shuffle _output_get)
  ;[1 1 1] This is used to direct which  set piece to spawn.
  (switch int (Math|Random|RandomInteger 7)
    (:0
      ;[1 1 1] Always connect the set piece with the relative transform node to make sure the obstacles appear above the floor.
      (AddComponent|AddChildActorComponent false (Math|Transform|MakeRelativeTransform (Utilities|Array|Get(acopy) (LocalVariables|GetRandom%20Spawn%20Points)) (Transformation|GetActorTransform))))
    (:1
      (AddComponent|AddChildActorComponent false (Math|Transform|MakeRelativeTransform (Utilities|Array|Get(acopy) (LocalVariables|GetRandom%20Spawn%20Points)) (Transformation|GetActorTransform))))
    (:2
      (AddComponent|AddChildActorComponent false (Math|Transform|MakeRelativeTransform (Utilities|Array|Get(acopy) (LocalVariables|GetRandom%20Spawn%20Points)) (Transformation|GetActorTransform))))
    (:3
      (AddComponent|AddChildActorComponent false (Math|Transform|MakeRelativeTransform (Utilities|Array|Get(acopy) (LocalVariables|GetRandom%20Spawn%20Points)) (Transformation|GetActorTransform))))
    (:4
      (AddComponent|AddChildActorComponent false (Math|Transform|MakeRelativeTransform (Utilities|Array|Get(acopy) (LocalVariables|GetRandom%20Spawn%20Points)) (Transformation|GetActorTransform))))
    (:5
      (AddComponent|AddChildActorComponent false (Math|Transform|MakeRelativeTransform (Utilities|Array|Get(acopy) (LocalVariables|GetRandom%20Spawn%20Points)) (Transformation|GetActorTransform))))
    (:6
      (AddComponent|AddChildActorComponent false (Math|Transform|MakeRelativeTransform (Utilities|Array|Get(acopy) (LocalVariables|GetRandom%20Spawn%20Points)) (Transformation|GetActorTransform))))))