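; Base obstacle Blueprint for the runner game, configured by a mesh asset and an obstacle type.
; The construction script applies the mesh, then maps Blockers to the WorldStatic object type and UnderRolls to PhysicsBody.
; SetUpBehavior applies that type with query-only collision that blocks Pawns, so the object channel is what distinguishes the two obstacle kinds.
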(fn ConstructionScript
  (Components|StaticMesh|SetStaticMesh (Variables|Default|GetStaticMesh) (Variables|AssetDatabase|GetStaticMeshAsset))
  (CallFunction|SetUpBehavior (Utilities|Select :Index (Variables|AssetDatabase|GetObstacleType) :NewEnumerator0 "ECC_WorldStatic" :NewEnumerator1 "ECC_PhysicsBody")))

(fn SetUpBehavior
  (params (Channel :type ECollisionChannel%20Enum :default "ECC_WorldStatic"))
  (bind _staticmesh (Variables|Default|GetStaticMesh))
  (Collision|SetCollisionEnabled _staticmesh "QueryOnly")
  (Collision|SetCollisionObjectType _staticmesh Channel)
  (Collision|SetCollisionResponsetoChannel _staticmesh "ECC_Pawn" "ECR_Block"))