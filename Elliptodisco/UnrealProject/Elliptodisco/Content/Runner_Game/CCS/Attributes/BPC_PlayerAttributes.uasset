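; Player attributes component that plays looping random emote montages on its owner's skeletal mesh in the Character Selection Screen.
; It caches the owner's skeletal mesh component on BeginPlay.
; EmoteNow plays a random montage from Emotes, then waits and repeats while CanEmote stays true.
; EmoteEnd clears the flag and blends out the active montage, such as when another menu opens.
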(event Custom|Emote%20End
  (bind _sk_component (Variables|Default|GetSK_Component))
  (bind _returnvalue (Components|SkeletalMesh|GetAnimInstance _sk_component))
  ;[0.15 0.15 0.15 0.5] Stop Emoting when another menu is opened. Similar method can be used for more context-aware menu interactions.
  (Variables|DoNotChange|SetCanEmote false)
  (Animation|Montage|MontageStop _returnvalue (Variables|Properties|Emotes|GetMontage%20Blend%20Out%20Time) (Animation|Montage|GetCurrentActiveMontage _returnvalue)))

(event Custom|Emote%20Now
  (Variables|DoNotChange|SetCanEmote true)
  ;[0.15 0.15 0.15 0.5] Keep Emoting as long as standing in Character Selection Screen
  (Animation|Montage|PlayMontage (Variables|Default|GetSK_Component) (.OutItem (Utilities|Array|Random (Variables|Properties|Emotes|GetEmotes))) :!label _label
    (:OnCompleted
      (Utilities|FlowControl|Delay (Variables|Properties|Emotes|GetWaitingTimeBeforeNextEmote))
      (if (Variables|DoNotChange|GetCanEmote)
        (goto _label)))))

(event EventBeginPlay
  ;[0.15 0.15 0.15 0.5] Cache once, use infinitely.
  (Variables|Default|SetSK_Component (Actor|GetComponentbyClass (Components|GetOwner) "/Script/Engine.SkeletalMeshComponent")))